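; AI_master_Bp is an AI Blueprint that holds health and receives bone-aware damage.
; On BeginPlay it fills CurrentHealth from MaxHealth and registers itself as owner of the AI_Hud in its widget component.
; The ITakeDamage event zeroes health on a Head bone hit and otherwise subtracts the damage, printing debug text either way.
; It contains no death handling or clamping of health.
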(event `self.ReceiveBeginPlay`
  (set `self.CurrentHealth` (`self.MaxHealth`))
  (bind _asai_hud (cast `/Game/AIBlueprint/AI_Hud` (`WidgetComponent.GetUserWidgetObject` (`self.Widget`))))
  (set `/Game/AIBlueprint/AI_Hud.Owner` self _asai_hud))

(event `/Game/AIBlueprint/TaskDamage.ITakeDamage`
  (params (BoneName :type Name) (Damage :type "Float (single-precision)"))
  (if (== BoneName "Head")
    (`KismetSystemLibrary.PrintString` "HeadShot" true true (struct :`R` 0.903692 :`G` 1.0 :`B` 0.917903 :`A` 1.0) 1.0)
    (set `self.CurrentHealth` 0.0)
    (else
      (set `self.CurrentHealth` (- (`self.CurrentHealth`) Damage))
      (`KismetSystemLibrary.PrintString` (`KismetStringLibrary.Conv_DoubleToString` Damage) true true (struct :`R` 0.903692 :`G` 1.0 :`B` 0.917903 :`A` 1.0) 1.0))))

(fn `UserConstructionScript`)